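; BP_Lamp_Blue is a blue lamp that blinks its point light a limited number of times when play begins.
; BeginPlay loops through a DoN node capped by Repeat, calling the blink event and waiting twice Speed between passes.
; Each blink switches the light on, off after a Speed delay, then on again after another.
; The on and off events set the light's visibility and track it in OnOffLight.
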(event `On_Light`
  (`SceneComponent.SetVisibility` (`self.PointLight`) true false)
  (set `self.On/Off_Light` true))

(event `Off_Light`
  (`SceneComponent.SetVisibility` (`self.PointLight`) false false)
  (set `self.On/Off_Light` false))

(event `Logic_Light_Blue`
  (bind _speed (`self.Speed`))
  (`self.On_Light`)
  (`KismetSystemLibrary.Delay` (stale _output_get))
  (`self.Off_Light`)
  (bind _output_get (set `self.Speed` _speed))
  (`KismetSystemLibrary.Delay` _speed)
  (`self.On_Light`))

(event `self.ReceiveBeginPlay`
  (`/Engine/EditorBlueprintResources/StandardMacros.Do N` (`self.Repeat`) :!label _label
    (:`Exit`
      (`self.Logic_Light_Blue`)
      (`KismetSystemLibrary.Delay` (* (`self.Speed`) 2.0))
      (goto _label))))

(fn `UserConstructionScript`)